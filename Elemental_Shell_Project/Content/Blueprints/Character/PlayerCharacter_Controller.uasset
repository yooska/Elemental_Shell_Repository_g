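; Player controller that spawns and possesses the FPS character on BeginPlay, passing it weapon, abilities, chassis, core and a randomly offset team and color.
; RespawnEvent kills the controlled pawn and spawns a replacement, so a weapon set through SetWeapon applies on the next spawn.
; It also creates the HUD and main menu, toggles the menu with Tab, and plays recoil camera shake.
; Loadout checking and spawn point selection are unfinished stubs.
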(event Custom|WalkShake)

(event Custom|Recoil%20Start
  (params (Intensity :type Float%20%28single-precision%29))
  ;[1 1 1] WeaponShake
  (Class|PlayerController|ClientPlayCameraShake (Variables|Default|GetCameraShake_Weapon) Intensity "CameraLocal" "0, 0, 0"))

(event Custom|SetWeapon
  (params (WeaponToSelect :type WeaponTypes%20Enum :default "NewEnumerator1"))
  ;[1 1 1] Have Menu allow players to set optionsthat are called next time the player pawn spawns
  (Variables|Default|SetWeaponType WeaponToSelect))

(event Custom|SpawnPlayerCharacter
  (bind _returnvalue (Math|Random|RandomIntegerinRange 0 3))
  (bind _self self)
  (bind _myteam (Variables|Default|GetMyTeam))
  (bind _returnvalue_2 (+ _myteam _returnvalue))
  (CallFunction|CheckLoadout)
  (bind _returnvalue_3 (Game|SpawnActorfromClass "/Game/Blueprints/Character/FPSCharacter_BP.FPSCharacter_BP_C" (Transformation|GetWorldTransform (Variables|Default|GetSpawnTransform)) "AdjustIfPossibleButAlwaysSpawn" _self _self (Variables|Default|GetCoreType) (Utilities|Array|Get(acopy) (Variables|Default|GetTeamColor) _returnvalue_2) (Variables|Default|GetAbilityPrimaryType) (Variables|Default|GetAbilitySecondaryType) _returnvalue_2 (Variables|Default|GetWeaponType) (Variables|Default|GetChassisType) 0))
  (Pawn|Possess _returnvalue_3))

(event Custom|FindSpawnPoints
  (bind _outactors (Actor|GetAllActorsOfClass "/Game/Blueprints/Character/SpawnPoint.SpawnPoint_C"))
  (bind _output_get (Variables|Default|SetSpawnPoints _outactors))
  (for _array_element _output_get
    _))

(event Custom|RespawnEvent
  (bind _asfpscharacter_bp (Utilities|Casting|CastToFPSCharacter_BP (Pawn|GetControlledPawn)))
  (Default|Die _asfpscharacter_bp)
  (CallFunction|SpawnPlayerCharacter))

(event Custom|CheckLoadout)

(event EventBeginPlay
  (bind _returnvalue (Game|GetPlayerController 0))
  (CallFunction|SpawnPlayerCharacter)
  ;[1 1 1] Create Main Menu
  (bind _returnvalue_2 (UserInterface|CreateWidget "/Game/Blueprints/Weapons/Game_HUD.Game_HUD_C" _returnvalue))
  (UserInterface|Viewport|AddtoViewport _returnvalue_2 0)
  (bind _returnvalue_3 (UserInterface|CreateWidget "/Game/Blueprints/Character/MainMenu.MainMenu_C" _returnvalue self))
  (UserInterface|Viewport|AddtoViewport _returnvalue_3 0))

(event Input|KeyboardEvents|Tab
  (params (Key :type Key%20Structure :default "None"))
  ;[1 1 1] Create Main Menu
  ;;[1 1 1] Toggle Menu Visibility
  (:Pressed
    (Utilities|FlowControl|FlipFlop
      (:A
        (Widget|SetVisibility (stale EventBeginPlay _returnvalue_3) "Visible"))
      (:B
        (Widget|SetVisibility (stale EventBeginPlay _returnvalue_3) "Hidden")))))

(fn ConstructionScript)