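; Player spirit character that flies along the camera direction and can possess physics objects or pawns.
; A looping timer line-traces for targets; the secondary action toggles possession, pausing the trace, disabling movement and using timelines to lerp location and spring-arm length.
; While possessing, holding the main action locks pitch and draws a debug predicted projectile path.
; Launching is unfinished: force is tracked but never applied, and the transparent-material swap is disconnected.
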(event OnComponentHit(Mesh)
  (params (HitComponent :type Primitive%20Component%20Object%20Reference) (OtherActor :type Actor%20Object%20Reference) (OtherComp :type Primitive%20Component%20Object%20Reference) (NormalImpulse :type Vector :default "0, 0, 0") (Hit :type Hit%20Result%20Structure%20%28by%20ref%29))
  (bind _possessedobject (Variables|Default|GetPossessedObject))
  (if (== OtherActor "/Game/Blueprints/Character/FPSCharacter_BP.FPSCharacter_BP")
    (Timeline|CalculateCurrentForce Stop ; play from when object is launch until it hits something
      (:Update
        (Variables|Default|SetDamageToDeal (* (Math|Vector|VectorLength (Transformation|GetVelocity _possessedobject)) (Physics|GetMass (Variables|/Script/Engine.StaticMeshActor|GetStaticMeshComponent _possessedobject))))))))

(event Custom|Trace%20For%20Possessable%20Object
  (bind _capsulecomponent (Variables|Collision|GetCapsuleComponent))
  (bind _returnvalue (Transformation|GetWorldLocation _capsulecomponent))
  (bind (_outhit _returnvalue_2) (Collision|LineTraceForObjects _returnvalue (+ (* (Math|Vector|GetForwardVector (Variables|Default|GetCamera)) (Variables|Default|GetPossessionRange)) _returnvalue) (Utilities|Array|MakeArray "ObjectTypeQuery4" "ObjectTypeQuery3") false 0 "ForDuration" true "(R=1.000000,G=0.000000,B=0.000000,A=1.000000)" "(R=0.000000,G=1.000000,B=0.000000,A=1.000000)" 3.0))
  (if _returnvalue_2
    (Variables|Default|SetPossessedActorTransform (Transformation|GetActorTransform (.HitActor (Collision|BreakHitResult _outhit))))
    (Variables|Default|SetMesh%20to%20Possess (.HitActor (Collision|BreakHitResult _outhit)))
    (Variables|Default|SetCanPossess true)
    (Utilities|FlowControl|Delay 0.25)
    (Development|PrintString (Utilities|String|Append "Can Possess:  " (Utilities|GetDisplayName (.HitComponent (Collision|BreakHitResult _outhit)))) true true "(R=0.050572,G=1.000000,B=0.000000,A=1.000000)")
    (else
      (Variables|Default|SetCanPossess false))))

(event Custom|Possess
  (params (PossessedObject :type Static%20Mesh%20Actor%20Object%20Reference))
  (Variables|Default|SetPossessedObject PossessedObject)
  (Pawn|Components|CharacterMovement|DisableMovement (Variables|Character|GetCharacterMovement))
  (Utilities|FlowControl|Sequence
    (:then_0
      (bind _lerptoposition (Timeline|LerpToObject%20Position Play)
        (:Update
          (Transformation|SetActorLocation self (.location (Math|Transform|Lerp(Transform) (Transformation|GetWorldTransform (Variables|Collision|GetCapsuleComponent)) (Variables|Default|GetPossessedActorTransform) _lerptoposition)) false false))))
    (:then_1
      (bind _updatespringlength (Timeline|SpringArmDistance Play)
        (:Update
          (Variables|/Script/Engine.SpringArmComponent|SetTargetArmLength (Variables|Default|GetSpringArm) _updatespringlength))))))

(event Custom|Unpossess
  (bind _savedmaterials (Variables|Default|GetSavedMaterials))
  (Utilities|FlowControl|Sequence
    (:then_0
      (Pawn|Components|CharacterMovement|SetMovementMode (Variables|Character|GetCharacterMovement) "MOVE_Flying" 0)
      (Transformation|DetachFromActor "KeepWorld" "KeepWorld" "KeepWorld")
      ;[1 1 1] Turn Mats transparent when possessed (only to possessing player) and turn them back to normal when unpossessing
      (for (_ _array_index) _savedmaterials
        (Rendering|Material|SetMaterial (Variables|/Script/Engine.StaticMeshActor|GetStaticMeshComponent (Variables|Default|GetPossessedObject)) _array_index (Utilities|Array|Get(acopy) _savedmaterials _array_index))))
    (:then_1
      (bind _updatespringlength (Timeline|SpringArmDistance Reverse)
        (:Update
          (Variables|/Script/Engine.SpringArmComponent|SetTargetArmLength (Variables|Default|GetSpringArm) _updatespringlength))))
    (:then_2
      (bind _lerptoposition (Timeline|LerpToObject%20Position Reverse)
        (:Update
          (Transformation|SetActorLocation self (.location (Math|Transform|Lerp(Transform) (Transformation|GetWorldTransform (Variables|Collision|GetCapsuleComponent)) (Variables|Default|GetPossessedActorTransform) _lerptoposition)) false false))))))

(event Custom|InitializePossessedActor
  (Transformation|AttachActorToActor self (Variables|Default|GetPossessedObject) "None" "SnapToTarget" "SnapToTarget" "SnapToTarget" true))

(event EventBeginPlay
  (bind _particlespawner (Variables|Default|GetParticleSpawner))
  (bind _returnvalue (Utilities|Time|SetTimerbyEvent (delegate Custom|Trace%20For%20Possessable%20Object) 0.1 true))
  (Utilities|FlowControl|Delay 2.0)
  (Effects|SpawnEmitterAttached "/Game/SuperGrid/TutorialLevel/Particles/P_Portal.P_Portal" _particlespawner "None" (Variables|/Script/Engine.SceneComponent|GetRelativeLocation _particlespawner) (Variables|/Script/Engine.SceneComponent|GetRelativeRotation _particlespawner) "0.700000,0.700000,0.700000"))

(event Input|ActionEvents|InputActionJump
  (params (Key :type Key%20Structure :default "None"))
  ;[1 1 1] Raise Character
  (:Pressed
    (Timeline|JumpingTimeline Play
      (:Update
        (Pawn|Input|AddMovementInput "0,0.000000,1.000000" 1.0 false))))
  (:Released
    (Timeline|JumpingTimeline Stop)))

(event Input|ActionEvents|InputActionActionSecondary
  (params (Key :type Key%20Structure :default "None"))
  (:Pressed
    (if (Variables|Default|GetCanPossess)
      (Utilities|FlowControl|FlipFlop
        (:A
          (Variables|Default|SetPossessingObject true)
          (Utilities|Time|PauseTimerbyHandle (stale EventBeginPlay _returnvalue))
          (Utilities|FlowControl|Delay 0.2)
          (CallFunction|Possess))
        (:B
          (Variables|Default|SetPossessingObject false)
          (Utilities|Time|UnpauseTimerbyHandle (stale EventBeginPlay _returnvalue))
          (CallFunction|Unpossess))))))

(event Input|ActionEvents|InputActionActionMain
  (params (Key :type Key%20Structure :default "None"))
  (:Pressed
    (if (Variables|Default|GetPossessingObject)
      (Variables|Default|SetChargingObjectForLaunch true)
      (Utilities|FlowControl|Sequence
        (:then_1
          (Timeline|ShowProjectilePath Play
            (:Update
              (Class|GameplayStatics|BlueprintPredictProjectilePathbyTraceChannel (Transformation|GetWorldLocation (Variables|Collision|GetCapsuleComponent)) (* (Math|Vector|GetForwardVector (Variables|Default|GetCamera)) 1e+03) true 5.0 "ECC_WorldStatic" false (Utilities|Array|MakeArray self) "ForDuration" 1.0) ; Use Out path positions to make some sort of visual effect
            ))))))
  (:Released
    (Variables|Default|SetChargingObjectForLaunch false)
    (Timeline|ShowProjectilePath Stop)))

(event Input|AxisEvents|InputAxisMouseLookVertical
  (params (AxisValue :type Float%20%28single-precision%29))
  ;[1 1 1] Mouse Look
  (if (not (Variables|Default|GetChargingObjectForLaunch))
    (if (Variables|Default|GetPossessingObject)
      _
      (else
        _))
    (Pawn|Input|AddControllerPitchInput AxisValue)
    (bind _output_get (Variables|Default|SetLaunchForce (+ (* AxisValue -1.0) (Variables|Default|GetLaunchForce))))
    (Development|PrintString (Utilities|String|ToString(Float) (* _output_get 1e+02)) false true "(R=1.000000,G=0.945536,B=0.159277,A=1.000000)")))

(event Input|AxisEvents|InputAxisMovementVertical
  (params (AxisValue :type Float%20%28single-precision%29))
  ;[1 1 1] Flying In Camera Direction
  (Pawn|Input|AddMovementInput (Math|Vector|GetForwardVector (Variables|Default|GetCamera)) AxisValue false))

(event Input|AxisEvents|InputAxisMouseLookHorizontal
  (params (AxisValue :type Float%20%28single-precision%29))
  ;[1 1 1] Mouse Look
  (if (Variables|Default|GetPossessingObject)
    _
    (else
      _))
  (Pawn|Input|AddControllerYawInput AxisValue))

(event Input|AxisEvents|InputAxisMovementHorizontal
  (params (AxisValue :type Float%20%28single-precision%29))
  ;[1 1 1] Flying In Camera Direction
  (Pawn|Input|AddMovementInput (Math|Vector|GetRightVector (Variables|Default|GetCamera)) AxisValue false))

(fn ConstructionScript)