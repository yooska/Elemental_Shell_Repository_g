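; Ability actor that lets a player aim a surface marker and grow a pillar there.
; CastAbility toggles the decal, with a Timeline tracing from the camera to align it to the surface normal.
; On confirmation it spawns AB_Pillar, routed through an authority check and request event, then scales it along a vector curve.
; Decal recoloring is marked not working, and PillarHit only prints, with its launch disconnected.
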(event Custom|InitializeAbility
  (params (PlayerCharacter :type FPS%20Character%20BP%20Object%20Reference) (Camera :type Camera%20Component%20Object%20Reference))
  (Variables|Default|SetPlayerCharacter PlayerCharacter)
  (Variables|Default|SetCamera Camera))

(event Custom|CastAbility
  (bind _camera (Variables|Default|GetCamera))
  (bind _returnvalue (Transformation|GetWorldLocation _camera))
  (bind _isa (Utilities|FlowControl|FlipFlop :!label _label)
    (:A
      _)
    (:B
      _))
  (Variables|Default|SetAbilityBeingCast _isa)
  (Variables|Default|SetDecalVisibilty _isa)
  (Rendering|SetVisibility (Variables|Default|GetAbilityMarker) (Variables|Default|GetDecalVisibilty) false)
  (if (Variables|Default|GetDecalVisibilty)
    (Timeline|Timeline_0 Play
      (:Update
        (bind _outhit (Collision|LineTraceByChannel _returnvalue (+ (* (Math|Vector|GetForwardVector _camera) 4e+03) _returnvalue) "TraceTypeQuery1" false 0 "ForOneFrame" true "(R=0.000000,G=1.000000,B=1.000000,A=1.000000)" "(R=0.916948,G=0.000000,B=1.000000,A=1.000000)")) ; Could use a cone cast or a square/capsule/etc Line trace\nUsing the cone random shot and getting the MEAN of the collective normals as the rotation/angle to cast from. Would make the circle slightly offset though? Or maybe that's fine. Worth testing
        (if (.bBlockingHit (Collision|BreakHitResult _outhit))
          (Transformation|SetWorldLocationAndRotation (Variables|Default|GetAbilityMarker) (.Location (Collision|BreakHitResult _outhit)) (Math|Rotator|MakeRotationfromAxes (.ImpactNormal (Collision|BreakHitResult _outhit)) "0, 0, 0" "0, 0, 0") false false)
          (if (Variables|Default|GetConfirmedAbilityUsage)
            (Utilities|FlowControl|Sequence
              (:then_0
                (goto _label))
              (:then_1
                (Variables|Default|SetDecalVisibilty true)
                ;[1 0.3073 0.3073 0.5] Not Working ATM: look into dynamic mats + make custom PNG
                (bind _returnvalue_2 (Rendering|Material|CreateDynamicMaterialInstance (Class|DecalComponent|GetDecalMaterial (Variables|Default|GetAbilityMarker)) "None" :!class /Script/Engine.KismetMaterialLibrary))
                (bind _returnvalue_3 (Rendering|Material|GetVectorParameterValue _returnvalue_2 "Color" :!class /Script/Engine.MaterialInstanceDynamic))
                (Class|OculusFunctionLibrary|SetColorScaleandOffset _returnvalue_3 "(R=0.000000,G=1.000000,B=0.179393,A=1.000000)" false)
                (Development|PrintString "something happens" true true "(R=0.000000,G=0.017204,B=1.000000,A=1.000000)")
                (Networking|SwitchHasAuthority
                  (:Authority
                    (CallFunction|SpawnPillarMC))
                  (:Remote
                    (CallFunction|SpawnPillarRQ)))))))))
    (else
      (Timeline|Timeline_0 Stop))))

(event Custom|PillarHit
  (params (LaunchDirection :type Vector))
  ;[1 1 1] Should pillar hurt player (can't use it to pop up now)
  (Development|PrintString "PillarHIT" true true "(R=1.000000,G=0.948081,B=0.906830,A=1.000000)"))

(event Custom|Spawn%20Pillar%20MC
  (bind _abilitymarker (Variables|Default|GetAbilityMarker))
  (bind _returnvalue (Transformation|GetWorldTransform _abilitymarker))
  (bind (_x _y _z) (Math|Vector|BreakVector (.location _returnvalue)))
  (bind _output_get (Variables|Default|SetPillarTransform (Math|Transform|MakeTransform (Math|Vector|MakeVector _x _y _z) (.rotation _returnvalue) "0.100000,0.100000,0.100000")))
  (bind _returnvalue_2 (Game|SpawnActorfromClass "/Game/Blueprints/Abilities/AB_Pillar.AB_Pillar_C" _output_get "Undefined" 0 0)) ; Could have it so if you do something like hold down the normal it changes to a cone test and grows towards the player? \nWill that actually work or will that only work on corners?\nIf it only works on corners that might actually be perfect
  (Utilities|FlowControl|Delay 0.5)
  (Variables|Default|SetDecalVisibilty false)
  (bind _pillarsizeincrease (Timeline|Timeline_1 PlayFromStart) ; Can edit the vector curve inside to set unique scaling speed
    (:Update
      (Transformation|SetWorldScale3D (Variables|/Game/Blueprints/Abilities/AB_Pillar.AB_Pillar_C|GetPillar _returnvalue_2) _pillarsizeincrease))
    (:Finished
      (Utilities|FlowControl|Delay 0.1)
      (Timeline|Timeline_1 Stop))))

(event Custom|Spawn%20Pillar%20RQ
  (CallFunction|SpawnPillarMC))

(event EventBeginPlay)

(event Collision|EventActorBeginOverlap
  (params (OtherActor :type Actor%20Object%20Reference)))

(event EventTick
  (params (DeltaSeconds :type Float%20%28single-precision%29)))

(event Input|KeyboardEvents|Q
  (params (Key :type Key%20Structure :default "None")))

(fn ConstructionScript)