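; AB_LaunchPad is an ability launch pad that notifies player characters when they overlap it.
; BeginPlay gathers actors tagged "Player", and the LaunchPad component's overlap event checks the entering actor against that list.
; A match that casts to FPSCharacter_BP receives PillarHit with the sweep impact point, leaving the response to the character, and debug prints report the cast result.
; An unconnected physics-impulse branch never runs.
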(event OnComponentBeginOverlap(LaunchPad)
  (params (OverlappedComponent :type Primitive%20Component%20Object%20Reference) (OtherActor :type Actor%20Object%20Reference) (OtherComp :type Primitive%20Component%20Object%20Reference) (OtherBodyIndex :type Integer) (bFromSweep :type Boolean) (SweepResult :type Hit%20Result%20Structure%20%28by%20ref%29))
  (for _array_element (stale EventBeginPlay _outactors)
    (if (== OtherActor _array_element)
      (bind _asfpscharacter_bp (Utilities|Casting|CastToFPSCharacter_BP _array_element)
        (:then
          (Default|PillarHit _asfpscharacter_bp (.ImpactPoint (Collision|BreakHitResult SweepResult)))
          (Development|PrintString "pillarcast"))
        (:CastFailed
          (Development|PrintString "failedcast"))))))

(event EventBeginPlay
  (bind _outactors (Actor|GetAllActorswithTag "Player")))

(fn ConstructionScript)