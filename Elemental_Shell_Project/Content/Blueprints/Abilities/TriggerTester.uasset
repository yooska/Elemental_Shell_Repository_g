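; TriggerTester is a test trigger actor that recolors the player while they overlap its Box component.
; On begin overlap by the first player's pawn, it calls ChangeColor on FPSCharacter_BP with a hard-coded red.
; On end overlap, it restores the character's PlayerBaseColor through the same call.
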(event OnComponentBeginOverlap(Box)
  (params (OverlappedComponent :type Primitive%20Component%20Object%20Reference) (OtherActor :type Actor%20Object%20Reference) (OtherComp :type Primitive%20Component%20Object%20Reference) (OtherBodyIndex :type Integer) (bFromSweep :type Boolean) (SweepResult :type Hit%20Result%20Structure%20%28by%20ref%29))
  (bind _returnvalue (Game|Player|GetPlayerPawn 0))
  (if (== OtherActor _returnvalue)
    (Default|ChangeColor (.AsFPSCharacter%20BP (Utilities|Casting|CastToFPSCharacter_BP _returnvalue)) "(R=1.000000,G=0.034709,B=0.000000,A=1.000000)")))

(event OnComponentEndOverlap(Box)
  (params (OverlappedComponent :type Primitive%20Component%20Object%20Reference) (OtherActor :type Actor%20Object%20Reference) (OtherComp :type Primitive%20Component%20Object%20Reference) (OtherBodyIndex :type Integer))
  (bind _returnvalue (Game|Player|GetPlayerPawn 0))
  (bind _asfpscharacter_bp (Utilities|Casting|CastToFPSCharacter_BP _returnvalue))
  (if (== OtherActor _returnvalue)
    (Default|ChangeColor _asfpscharacter_bp (Variables|/Game/Blueprints/Character/FPSCharacter_BP.FPSCharacter_BP_C|GetPlayerBaseColor _asfpscharacter_bp))))

(event EventBeginPlay)

(event Collision|EventActorBeginOverlap
  (params (OtherActor :type Actor%20Object%20Reference)))

(event EventTick
  (params (DeltaSeconds :type Float%20%28single-precision%29)))

(fn ConstructionScript)