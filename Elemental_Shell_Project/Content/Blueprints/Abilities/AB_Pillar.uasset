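; AB_Pillar is an ability pillar that hardens after spawning, with a comment noting it becomes wall-runnable.
; BeginPlay disables overlap events on Pillar, then after a short delay swaps its material and re-enables them.
; A second component, Pillar2, passes overlap impact points to FPSCharacter_BP's PillarHit.
; Pillar's hit handler only prints debug text, and unconnected experiments for tag lookup and impulses remain.
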(event OnComponentHit(Pillar)
  (params (HitComponent :type Primitive%20Component%20Object%20Reference) (OtherActor :type Actor%20Object%20Reference) (OtherComp :type Primitive%20Component%20Object%20Reference) (NormalImpulse :type Vector :default "0, 0, 0") (Hit :type Hit%20Result%20Structure%20%28by%20ref%29))
  ;[1 1 1] just use this method... LEANRING
  (bind _asfpscharacter_bp (Utilities|Casting|CastToFPSCharacter_BP OtherActor))
  (Utilities|FlowControl|Delay 0.2)
  (Development|PrintString "Hello"))

(event OnComponentBeginOverlap(Pillar2)
  (params (OverlappedComponent :type Primitive%20Component%20Object%20Reference) (OtherActor :type Actor%20Object%20Reference) (OtherComp :type Primitive%20Component%20Object%20Reference) (OtherBodyIndex :type Integer) (bFromSweep :type Boolean) (SweepResult :type Hit%20Result%20Structure%20%28by%20ref%29))
  (bind (_bblockinghit _binitialoverlap _time _distance _location _impactpoint _normal _impactnormal _physmat _hitactor) (Collision|BreakHitResult SweepResult))
  (bind _asfpscharacter_bp (Utilities|Casting|CastToFPSCharacter_BP _hitactor)
    (:then
      (Development|PrintString "Hello")
      (Default|PillarHit 0 _impactpoint)
      (Development|PrintString "pillarcast"))
    (:CastFailed
      (Development|PrintString "failedcast"))))

(event EventBeginPlay
  (bind _pillar (Variables|Default|GetPillar))
  (Variables|/Script/Engine.PrimitiveComponent|SetbGenerateOverlapEvents _pillar false)
  ;[1 1 1] Material hardens and becomes wall-runnable
  (Utilities|FlowControl|Delay 1.5)
  (Rendering|Material|SetMaterial _pillar 0 "/Game/SuperGrid/StarterPack/Materials/Base/M_SuperGrid_PanelCustom.M_SuperGrid_PanelCustom")
  (Variables|/Script/Engine.PrimitiveComponent|SetbGenerateOverlapEvents _pillar true))

(fn ConstructionScript)