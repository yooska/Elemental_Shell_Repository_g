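; Bullet projectile actor that scales its mesh and tracer just after spawning and destroys itself after a short lifetime.
; A blocking mesh hit on an FPSCharacter_BP passes body and headshot damage, impact point and attacking team to its TakeDamage, then destroys the bullet.
; Other hits leave it alive until timeout.
; Surface-based impact particles are unfinished: their branch is disconnected and both particle events are empty.
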(event OnComponentHit(BulletMesh)
  (params (HitComponent :type Primitive%20Component%20Object%20Reference) (OtherActor :type Actor%20Object%20Reference) (OtherComp :type Primitive%20Component%20Object%20Reference) (NormalImpulse :type Vector :default "0, 0, 0") (Hit :type Hit%20Result%20Structure%20%28by%20ref%29))
  (bind (_bblockinghit _binitialoverlap _time _distance _location _impactpoint) (Collision|BreakHitResult Hit))
  (if _bblockinghit
    (bind _asfpscharacter_bp (Utilities|Casting|CastToFPSCharacter_BP OtherActor)) ; may have to add additional effects for things such as shooting down "missiles"
    (Default|TakeDamage _asfpscharacter_bp (Variables|Default|GetDamage) (Variables|Default|GetHeadshotDamage) HitComponent _impactpoint (Variables|Default|GetAttackTeam))
    (Development|PrintString "Should have dealth damage" true true "(R=1.000000,G=0.574254,B=0.000000,A=1.000000)")
    (Actor|DestroyActor)))

(event Custom|Play%20Hit%20Particle%20MC
  ;[1 1 1] setup to play on server
)

(event Custom|Play%20Hit%20Particle
  ;[1 1 1] setup to play on server
)

(event EventBeginPlay
  (Utilities|FlowControl|Delay 0.01)
  (Transformation|SetWorldScale3D (Variables|Default|GetBulletMesh) "0.050000,0.050000,0.050000")
  (Transformation|SetWorldScale3D (Variables|Default|GetTracer) "0.500000,0.050000,0.050000")
  (Utilities|FlowControl|Delay 5.0)
  (Actor|DestroyActor))

(fn ConstructionScript)