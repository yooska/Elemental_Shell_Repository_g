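; An older weapon Blueprint that gathers weapon actors in the level and prints their names for on-screen or log output.
; On BeginPlay it stores all actors of the SelectedWeapon class in WeaponList and adds each one's WeaponInfo name to WeaponName.
; The print loop is nested, so the growing name list reprints after every addition.
; Disconnected rotation-check nodes, including a retriggerable delay and a full-turn offset, never run.
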(event EventBeginPlay
  (bind _weaponname (Variables|Default|GetWeaponName))
  (bind _outactors (Actor|GetAllActorsOfClass (Variables|Default|GetSelected%20Weapon)))
  (bind _output_get (Variables|Default|SetWeaponList _outactors))
  (for _array_element _output_get
    (Utilities|Array|Add _weaponname (.Name (Utilities|Struct|BreakWeaponStats (Variables|/Game/Blueprints/Weapons/WeaponBase.WeaponBase_C|GetWeaponInfo _array_element))))
    (for _array_element_2 _weaponname
      (Development|PrintString (Utilities|String|ToString(Name) _array_element_2)))))

(fn ConstructionScript)