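; Base weapon Blueprint that fires projectiles in semi-auto, burst or full-auto modes, configured from WeaponInfo.
; TriggerDown calls ShootWeapon, which consumes ammo and spawns a projectile with cone deviation, or clanks when empty.
; AimOffsetTrace traces from the camera so shots leave the barrel toward the crosshair, falling back to control rotation.
; Reload only starts an elapsed-time timer without refilling; animations are print placeholders and recoil logic is unconnected.
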(event Custom|ReloadTimer
  (Variables|Default|SetCurrentTimeInReload (+ (Variables|Default|GetCurrentTimeInReload) 0.1)))

(event Custom|InitializeValues
  (params (FPS_Character :type FPS%20Character%20BP%20Object%20Reference))
  (bind _output_get (Variables|Default|SetPlayer FPS_Character))
  (Variables|Default|SetPlayerCamera (Variables|/Game/Blueprints/Character/FPSCharacter_BP.FPSCharacter_BP_C|GetCamera _output_get)))

(event Custom|GetAimOffset
  (CallFunction|AimOffsetTrace (Variables|Default|GetPlayerCamera) (Variables|AimOffset|GetAim%20Offset%20Max%20Range) (Variables|Default|GetProjectileSpawnPoint)) ; Bullets fires from gun barrel but paths to players crosshair
)

(event Custom|TriggerUp
  (Variables|Default|SetTriggerPressed false))

(event Custom|Shoot%20Weapon
  (bind _weaponinfo (Variables|Default|GetWeaponInfo))
  (bind _aimtransform (Variables|AimOffset|GetAimTransform))
  (bind (_name _weaponclass _ammotype _firemode _burstdelay _burstrate _burstprojectileamount _firerate _muzzlevelocity _reloadeject _reloadtime _activereloadupperbounds _magazinesize _activereloadlowerbounds _specialproperties _horizontalrecoilmod _verticalrecoilmod _recoil _deviation) (Utilities|Struct|BreakWeaponStats _weaponinfo))
  (if (!= (Variables|Reload|GetCurrentMagAmount) 0)
    (CallFunction|GetAimOffset)
    (if (Variables|Default|GetAiming)
      ;[1 1 1 1 12] Access anim bp here. Could have multiple animations for recoil patterns and one is chosen at random. Have it just effect upper half of the body and then play different ones for whichever anim state/firing state it's working with
      (Development|PrintString "Anim_BP for weapon hipfire plays " false false)
      (else
        (Development|PrintString "Anim_BP for weapon aimed plays" false false)))
    (Game|SpawnActorfromClass "/Game/Blueprints/Weapons/Bullet.Bullet_C" (Math|Transform|MakeTransform (.location _aimtransform) (Math|Conversions|RotationFromXVector (Class|KismetMathLibrary|RandomUnitVectorinEllipticalConeinDegrees (Math|Rotator|GetRotationXVector (.rotation _aimtransform)) (* _deviation 1.0) (* _deviation 1.0))) "1,1,1") "Undefined" 0 _muzzlevelocity _ammotype false 0)
    (Variables|Reload|SetCurrentMagAmount (- (Variables|Reload|GetCurrentMagAmount) 1))
    (else
      (Audio|PlaySoundatLocation "/Game/SuperGrid/TutorialLevel/SoundEffects/MechClank.MechClank" (Transformation|GetWorldLocation (Variables|Default|GetGunMesh)) "0, 0, 0" 1.0 1.0 0.0 0 0 0)
      (Development|PrintString "Hello" false) ; Enable HUD element "r to reload"
    )))

(event Custom|TriggerDown
  (bind _weaponinfo (Variables|Default|GetWeaponInfo))
  (bind (_name _weaponclass _ammotype _firemode _burstdelay _burstrate _burstprojectileamount _firerate _muzzlevelocity _reloadeject _reloadtime _activereloadupperbounds _magazinesize _activereloadlowerbounds _specialproperties _horizontalrecoilmod _verticalrecoilmod _recoil _deviation _scopedrecoilreduction _scopeddeviationreduction _scopeintime _1handedrecoilincrease _1handeddeviationincrease _armorpenetration _2handedrecoilshake) (Utilities|Struct|BreakWeaponStats _weaponinfo))
  (Variables|Default|SetTriggerPressed true)
  (Variables|Reload|SetIsReloading false)
  (switch Utilities|FlowControl|Switch|SwitchonFireModes _firemode
    (:NewEnumerator0
      (Utilities|FlowControl|DoOnce false :!label _label
        (:Completed
          (Utilities|FlowControl|Sequence
            (:then_0
              (CallFunction|ShootWeapon))
            (:then_1
              (Utilities|FlowControl|RetriggerableDelay _firerate)
              (goto _label Reset))))))
    (:NewEnumerator1
      (Utilities|FlowControl|DoOnce false :!label _label_2
        (:Completed
          (Utilities|FlowControl|Sequence
            (:then_0
              (bind _counter (Utilities|FlowControl|DoN _burstprojectileamount :!label _label_3)
                (:Exit
                  (switch int _counter
                    (:0
                      (CallFunction|ShootWeapon)
                      (Utilities|FlowControl|Delay _burstrate)
                      (goto _label_3 Reset))))))
            (:then_1
              (Utilities|FlowControl|RetriggerableDelay 0.2)
              (goto _label_2 Reset))))))
    (:NewEnumerator2
      (Utilities|Time|SetTimerbyFunctionName self "ShootWeapon" _firerate (Variables|Default|GetTriggerPressed)))))

(event Custom|RecoilTester)

(event Custom|Reload
  (Utilities|Time|SetTimerbyEvent (delegate Custom|ReloadTimer) 0.1 (Variables|Reload|GetIsReloading)))

(event EventBeginPlay
  (bind _weaponinfo (Variables|Default|GetWeaponInfo))
  (bind (_name _weaponclass _ammotype _firemode _burstdelay _burstrate _burstprojectileamount _firerate _muzzlevelocity _reloadeject _reloadtime _activereloadupperbounds _magazinesize _activereloadlowerbounds _specialproperties _horizontalrecoilmod _verticalrecoilmod) (Utilities|Struct|BreakWeaponStats _weaponinfo))
  (Utilities|FlowControl|Sequence
    (:then_0
      (Variables|Default|SetFireRate _firerate))
    (:then_1
      (Variables|Reload|SetReloadEjectTime _reloadeject)
      (Variables|Reload|SetReloadTime _reloadtime)
      (Variables|Reload|SetAR_UpperBounds _activereloadupperbounds)
      (Variables|Reload|SetAR_LowerBounds _activereloadlowerbounds)
      (bind _output_get (Variables|Reload|SetMaxMagSize _magazinesize))
      (Variables|Reload|SetCurrentMagAmount _output_get))
    (:then_2
      (Variables|Default|SetHorizontalRecoilMod _horizontalrecoilmod)
      (Variables|Default|SetVerticalRecoilMod _verticalrecoilmod))))

(fn ConstructionScript)

(fn AimOffsetTrace
  (params (PlayerCamera :type Camera%20Component%20Object%20Reference) (Camera%20Max%20Trace :type Float%20%28single-precision%29) (Projectile%20Spawn%20Point :type Scene%20Component%20Object%20Reference))
  (bind _returnvalue (Transformation|GetWorldLocation PlayerCamera))
  (bind _returnvalue_2 (Math|Vector|GetForwardVector PlayerCamera))
  (bind _returnvalue_3 (Transformation|GetWorldLocation Projectile%20Spawn%20Point))
  (bind _returnvalue_4 (* _returnvalue_2 Camera%20Max%20Trace))
  (bind _returnvalue_5 (+ _returnvalue _returnvalue_4))
  (Variables|AimOffset|SetMax%20Range%20Hit%20Location _returnvalue_5)
  (bind (_outhit _returnvalue_6) (Collision|LineTraceByChannel _returnvalue _returnvalue_5 "TraceTypeQuery1" false 0 "ForOneFrame"))
  (if _returnvalue_6
    (Variables|AimOffset|SetAimOffsetHit true) ; Camera sees something to direct bullet towards
    (Variables|AimOffset|SetAimTransform (Math|Transform|MakeTransform _returnvalue_3 (Math|Rotator|MakeRotfromX (- (.ImpactPoint (Collision|BreakHitResult _outhit)) _returnvalue_3))))
    (else
      (Variables|AimOffset|SetAimOffsetHit false) ; Didn't detect the camera looking at a target, fire from barrel with no offset
      (Variables|AimOffset|SetAimTransform (Math|Transform|MakeTransform (Transformation|GetSocketLocation Projectile%20Spawn%20Point "None") (Pawn|GetControlRotation (Variables|Default|GetPlayer) :!class /Script/Engine.Pawn))))))